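; Worker character that wanders idly and, when sent to a point, runs there as a fire escape, with state mirrored to its animation Blueprint.
; BeginPlay adds the main UI widget and starts a wander loop of random nearby AI moves with pauses, which halts while fire is on and escape is incomplete.
; The moveToPoint event sets fire flags and speed, then marks the worker escaped on arrival.
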(event `moveToPoint`
  (params (targetLocation :type "Vector Structure" :default (-900.0 900.0 0.0)))
  (set `/Game/yjs/BluePrint/Worker_Man/Worker_Man_Anim_BP.isEscape` false (stale `MoveRandomly` _asworker_man_anim_bp))
  (set `/Game/yjs/BluePrint/Worker_Man/Worker_Man_Anim_BP.isFireOn` true (stale `MoveRandomly` _asworker_man_anim_bp))
  (set `CharacterMovementComponent.MaxWalkSpeed` 400.0 (`self.CharacterMovement`))
  (`|AIMoveTo` self targetLocation null 100.0
    (:`then`
      (set `/Game/yjs/BluePrint/Worker_Man/Worker_Man_Anim_BP.isFireOn` true (stale `MoveRandomly` _asworker_man_anim_bp)))
    (:`OnSuccess`
      (set `/Game/yjs/BluePrint/Worker_Man/Worker_Man_Anim_BP.isEscape` true (stale `MoveRandomly` _asworker_man_anim_bp))
      (set `/Game/yjs/BluePrint/Worker_Man/Worker_Man_Anim_BP.isWalking` false (stale `MoveRandomly` _asworker_man_anim_bp)))))

(event `MoveRandomly`
  (bind _asworker_man_anim_bp (cast `/Game/yjs/BluePrint/Worker_Man/Worker_Man_Anim_BP` (`SkeletalMeshComponent.GetAnimInstance` (`self.Mesh`)) :!label _label))
  (if (not (and (not (`/Game/yjs/BluePrint/Worker_Man/Worker_Man_Anim_BP.isEscape` _asworker_man_anim_bp)) (`self.FireOn`)))
    (set `/Game/yjs/BluePrint/Worker_Man/Worker_Man_Anim_BP.isWalking` true _asworker_man_anim_bp)
    (`|AIMoveTo` self (`NavigationSystemV1.K2_GetRandomReachablePointInRadius` (`self.K2_GetActorLocation`) 400.0 null null) null
      (:`OnSuccess`
        _)
      (:`OnFail`
        _))
    (set `/Game/yjs/BluePrint/Worker_Man/Worker_Man_Anim_BP.isWalking` false _asworker_man_anim_bp)
    (`KismetSystemLibrary.Delay` 2.0)
    (goto _label)))

(event `self.ReceiveBeginPlay`
  (bind _returnvalue (`|CreateWidget` "/Game/yjs/UI/Main_UI_BP.Main_UI_BP_C"))
  (`UserWidget.AddToViewport` _returnvalue 0)
  (`self.MoveRandomly`))

(fn `UserConstructionScript`)