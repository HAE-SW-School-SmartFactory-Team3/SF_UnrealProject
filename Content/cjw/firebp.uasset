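; Fire actor that grows steadily larger over time after spawning.
; BeginPlay starts a looping timer for IncreaseSize, which multiplies CurrentScale, prints it and applies it as a uniform actor scale.
; A SpreadFire function can spawn another Firebp at a fixed distance in a random 3D direction, but its looping timer is disconnected, so the fire does not spread.
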(event `self.ReceiveBeginPlay`
  (`KismetSystemLibrary.K2_SetTimer` null "IncreaseSize" 3.0 true))

(fn `IncreaseSize`
  (bind _currentscale (`self.CurrentScale`))
  (bind _output_get (set `self.CurrentScale` (* _currentscale 1.1)))
  (`KismetSystemLibrary.PrintString` (`KismetStringLibrary.Conv_DoubleToString` _currentscale))
  (`self.SetActorScale3D` (`KismetMathLibrary.MakeVector` _output_get _output_get _output_get)))

(fn `SpreadFire`
  (`|SpawnActorFromClass` "firebp_C" (`KismetMathLibrary.MakeTransform` (+ (`self.K2_GetActorLocation`) (* (`KismetMathLibrary.RandomUnitVector`) 200.0))) "Undefined" "MultiplyWithRoot" null null))

(fn `UserConstructionScript`)