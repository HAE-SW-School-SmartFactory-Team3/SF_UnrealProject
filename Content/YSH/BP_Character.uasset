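; Test character Blueprint that uses its AI controller to move toward actors in a reference array, starting on BeginPlay.
; The looping Test event marks and moves to the current target, re-issuing successful requests and switching to the nearest unmarked actor on failure.
; Already at Goal is unhandled there, ending the loop.
; An alternative round-robin event, CustomMovementCall, is never started, and AIMoveTo experiments remain disconnected.
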(event `self.ReceiveBeginPlay`
  (`self.test`))

(event `CustomMovementCall`
  (bind _returnvalue (`AIController.MoveToLocation` (`AIBlueprintHelperLibrary.GetAIController` self) (`self.K2_GetActorLocation` (`|GetArrayItem` (`self.ActorReference`) (`self.TargetIndex`))) 5.0 false true false true null false :!label _label))
  (switch `EPathFollowingRequestResult` _returnvalue
    (:`Failed`
      (`KismetSystemLibrary.PrintString` "Failed"))
    (:`AlreadyAtGoal`
      _)
    (:`RequestSuccessful`
      (`KismetSystemLibrary.Delay` 1.0)
      (goto _label)))
  (set `self.TargetIndex` (mod (+ (`self.TargetIndex`) 1) (`KismetArrayLibrary.Array_Length` (`self.ActorReference`))))
  (`KismetSystemLibrary.PrintString` "Success")
  (`KismetSystemLibrary.Delay` 1.0)
  (`self.CustomMovementCall`))

(event `test`
  (bind _targetindex (`self.TargetIndex`))
  (`KismetArrayLibrary.Array_Set` (`self.Referenced`) _targetindex true)
  (bind _returnvalue (`AIController.MoveToLocation` (`AIBlueprintHelperLibrary.GetAIController` self) (`self.K2_GetActorLocation` (`|GetArrayItem` (`self.ActorReference`) _targetindex)) 5.0 false true false true null false))
  (switch `EPathFollowingRequestResult` _returnvalue
    (:`Failed`
      (set `self.MinIndex` 0)
      (set `self.MinValue` 1000000000000000.0)
      (for (_array_element _array_index) (`self.ActorReference`)
        (if (not (`|GetArrayItem` (`self.Referenced`) _array_index))
          (bind _returnvalue_2 (`KismetMathLibrary.Vector_DistanceSquared` (`CharacterMovementComponent.GetLastUpdateLocation` (`self.CharacterMovement`)) (`self.K2_GetActorLocation` _array_element)))
          (if (> (`self.MinValue`) _returnvalue_2)
            (set `self.MinIndex` _array_index)
            (set `self.MinValue` _returnvalue_2)
            (`KismetArrayLibrary.Array_Set` (`self.Referenced`) 0 true))))
      (set `self.TargetIndex` (`self.MinIndex`))
      (`KismetSystemLibrary.Delay` 1.0)
      (`self.test`))
    (:`RequestSuccessful`
      (`KismetSystemLibrary.Delay` 0.2)
      (`self.test`))))

(fn `UserConstructionScript`)