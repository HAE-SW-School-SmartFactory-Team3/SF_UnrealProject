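; BP_Destination is an escape point that tallies Worker_Man_BP actors by health condition as they reach it.
; On overlap it sorts the worker by HP into normal, slight or serious injury, incrementing both its own Info array and BP_InfoManager's Infos, then destroys the worker.
; TextRendering refreshes per-category and total escape labels on its text renders.
; Every tick the actor rotates to face the player pawn, keeping the labels readable.
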(event `self.ReceiveTick`
  (params (DeltaSeconds :type "Float (single-precision)"))
  (`self.K2_SetActorRotation` (`KismetMathLibrary.FindLookAtRotation` (`SceneComponent.K2_GetComponentLocation` (`self.NormalTextRender`)) (`self.K2_GetActorLocation` (`GameplayStatics.GetPlayerPawn` 0)))))

(event `TextRendering`
  (`TextRenderComponent.K2_SetText` (`self.NormalTextRender`) (`KismetTextLibrary.Conv_StringToText` (`KismetStringLibrary.Concat_StrStr` "Normal : " (`KismetStringLibrary.Conv_IntToString` (`|GetArrayItem` (`self.Info`))))))
  (`TextRenderComponent.K2_SetText` (`self.SlightTextRender`) (`KismetTextLibrary.Conv_StringToText` (`KismetStringLibrary.Concat_StrStr` "Slight : " (`KismetStringLibrary.Conv_IntToString` (`|GetArrayItem` (`self.Info`) 1)))))
  (`TextRenderComponent.K2_SetText` (`self.SeriousTextRender`) (`KismetTextLibrary.Conv_StringToText` (`KismetStringLibrary.Concat_StrStr` "Serious : " (`KismetStringLibrary.Conv_IntToString` (`|GetArrayItem` (`self.Info`) 2)))))
  (`TextRenderComponent.K2_SetText` (`self.TotalTextRender`) (`KismetTextLibrary.Conv_StringToText` (`KismetStringLibrary.Concat_StrStr` "Total Escape : " (`KismetStringLibrary.Conv_IntToString` (+ (`|GetArrayItem` (`self.Info`)) (`|GetArrayItem` (`self.Info`) 1) (`|GetArrayItem` (`self.Info`) 2)))))))

(event `self.ReceiveActorBeginOverlap`
  (params (OtherActor :type "Actor Object Reference"))
  (bind _info (`self.Info`))
  (bind _info_2 (`self.Info`))
  (bind _info_3 (`self.Info`))
  (bind _asworker_man_bp (cast `/Game/ysh/Worker_Man_BP` OtherActor))
  (if (>= (`/Game/ysh/Worker_Man_BP.HP` _asworker_man_bp) 90)
    (`KismetArrayLibrary.Array_Set` _info_3 0 (+ (`|GetArrayItem` _info_3) 1))
    (`KismetSystemLibrary.PrintString` "정상")
    (bind _returnvalue (`GameplayStatics.GetActorOfClass` "/Game/ysh/BP_InfoManager.BP_InfoManager_C"))
    (bind _infos (`/Game/ysh/BP_InfoManager.Infos` _returnvalue))
    (`KismetArrayLibrary.Array_Set` _infos 0 (+ (`|GetArrayItem` _infos) 1))
    (`self.K2_DestroyActor` _asworker_man_bp :!label _label)
    (`self.TextRendering`)
    (elif (>= (`/Game/ysh/Worker_Man_BP.HP` _asworker_man_bp) 50)
      (`KismetArrayLibrary.Array_Set` _info_2 1 (+ (`|GetArrayItem` _info_2 1) 1))
      (`KismetSystemLibrary.PrintString` "경상")
      (bind _returnvalue_2 (`GameplayStatics.GetActorOfClass` "/Game/ysh/BP_InfoManager.BP_InfoManager_C"))
      (bind _infos_2 (`/Game/ysh/BP_InfoManager.Infos` _returnvalue_2))
      (`KismetArrayLibrary.Array_Set` _infos_2 1 (+ (`|GetArrayItem` _infos_2 1) 1))
      (goto _label)
      (elif (>= (`/Game/ysh/Worker_Man_BP.HP` _asworker_man_bp) 0)
        (`KismetArrayLibrary.Array_Set` _info 2 (+ (`|GetArrayItem` _info 2) 1))
        (`KismetSystemLibrary.PrintString` "중상")
        (bind _returnvalue_3 (`GameplayStatics.GetActorOfClass` "/Game/ysh/BP_InfoManager.BP_InfoManager_C"))
        (bind _infos_3 (`/Game/ysh/BP_InfoManager.Infos` _returnvalue_3))
        (`KismetArrayLibrary.Array_Set` _infos_3 2 (+ (`|GetArrayItem` _infos_3 2) 1))
        (goto _label)))))

(fn `UserConstructionScript`)