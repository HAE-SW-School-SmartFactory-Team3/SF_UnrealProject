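; Fire manager that starts a fire at StartFirePoint on FireOn and spreads it through the level.
; Each delayed pass sphere-traces WorldStatic near every BP_FIre2, newest-first, spawning another on a hit at a re-rolled random offset.
; Passes stop once CurrentSpread reaches MaxSpreadCount, which is checked only between passes.
; While Worker_Man_BP's FireOn flag is false, a looping timer blinks a BP_FirePoint marker at the start point.
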(event `FireOn`
  (`|SpawnActorFromClass` "/Game/ysh/Vefects/Free_Fire/Shared/Particles/BP_FIre2.BP_FIre2_C" (`KismetMathLibrary.MakeTransform` (`self.StartFirePoint`)) "Undefined" "MultiplyWithRoot" null null)
  (`self.FireManagement`))

(event `FireManagement`
  (`KismetSystemLibrary.Delay` (`self.SpreadDelay`) :!label _label)
  (if (< (`self.CurrentSpread`) (`self.MaxSpreadCount`))
    (bind _outactors (`GameplayStatics.GetAllActorsOfClass` "/Game/ysh/Vefects/Free_Fire/Shared/Particles/BP_FIre2.BP_FIre2_C"))
    (`KismetArrayLibrary.Array_Reverse` _outactors)
    (for (_array_element _array_index) _outactors
      (if (== _array_index 1000)
        (break)
        (else
          (bind _returnvalue (`KismetMathLibrary.MakeVector` (+ (.x (.location (`self.GetTransform` _array_element))) (`KismetMathLibrary.RandomFloatInRange` (* (`self.SpreadRangeRadius`) -1.0) (`self.SpreadRangeRadius`))) (+ (.y (.location (`self.GetTransform` _array_element))) (`KismetMathLibrary.RandomFloatInRange` (* (`self.SpreadRangeRadius`) -1.0) (`self.SpreadRangeRadius`))) (.z (.location (`self.GetTransform` _array_element)))))
          (bind (_outhits _returnvalue_2) (`KismetSystemLibrary.SphereTraceMultiForObjects` _returnvalue _returnvalue 10.0 (`|MakeArray` "ObjectTypeQuery1" :!type "EObjectTypeQuery Enum") false _outactors))
          (if _returnvalue_2
            (`|SpawnActorFromClass` "/Game/ysh/Vefects/Free_Fire/Shared/Particles/BP_FIre2.BP_FIre2_C" (`KismetMathLibrary.MakeTransform` _returnvalue (.rotation (`self.GetTransform` _array_element)) (.scale (`self.GetTransform` _array_element))) "AdjustIfPossibleButDontSpawnIfColliding" "MultiplyWithRoot" null null)
            (set `self.CurrentSpread` (+ (`self.CurrentSpread`) 1))))))
    (goto _label)))

(event `self.ReceiveBeginPlay`
  (`KismetSystemLibrary.K2_SetTimerDelegate` (delegate `CustomEvent`) 1.0 true))

(event `CustomEvent`
  (bind _returnvalue (`GameplayStatics.GetActorOfClass` "/Game/ysh/Worker_Man_BP.Worker_Man_BP_C"))
  (if (`/Game/ysh/Worker_Man_BP.FireOn` _returnvalue)
    _
    (elif (`self.FlickerFlag`)
      (`self.K2_DestroyActor` (stale _returnvalue_2))
      (set `self.FlickerFlag` false)
      (else
        (bind _returnvalue_2 (`|SpawnActorFromClass` "/Game/ysh/BP_FirePoint.BP_FirePoint_C" (`KismetMathLibrary.MakeTransform` (`self.StartFirePoint`)) "AlwaysSpawn" "MultiplyWithRoot" null null))
        (set `self.FlickerFlag` true)))))

(fn `UserConstructionScript`)