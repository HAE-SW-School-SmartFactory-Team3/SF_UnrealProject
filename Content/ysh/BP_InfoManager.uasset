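; BP_InfoManager is a debug readout that prints the first four entries of its Infos array.
; BeginPlay starts a looping half-second timer whose event converts those entries to strings, joins them and prints the result.
; The graphs only read Infos by fixed index and never fill it, and the construction script is empty.
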(event `self.ReceiveBeginPlay`
  (`KismetSystemLibrary.K2_SetTimerDelegate` (delegate `CustomEvent`) 0.5 true))

(event `CustomEvent`
  (`KismetSystemLibrary.PrintString` (`KismetStringLibrary.Concat_StrStr` (`KismetStringLibrary.Conv_IntToString` (`|GetArrayItem` (`self.Infos`))) (`KismetStringLibrary.Conv_IntToString` (`|GetArrayItem` (`self.Infos`) 1)) (`KismetStringLibrary.Conv_IntToString` (`|GetArrayItem` (`self.Infos`) 2)) (`KismetStringLibrary.Conv_IntToString` (`|GetArrayItem` (`self.Infos`) 3)))))

(fn `UserConstructionScript`)