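; BP_FIre2 is a fire actor that can spread by spawning copies of itself, with its Niagara effect paused five seconds after BeginPlay.
; StartFire marks it burning, activates the effect and calls SpawnNewFire, which immediately spawns copies at random XY offsets within SpreadRangeRadius until MaxSpreadCount is reached.
; Nothing here calls StartFire: the box overlap is empty, and the delayed ignition and destroy nodes are disconnected.
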(event `self.ReceiveBeginPlay`
  (`KismetSystemLibrary.Delay` 5.0)
  (`NiagaraComponent.SetPaused` (`self.NS_Fire`) true))

(event `self.Box.OnComponentBeginOverlap`
  (params (OverlappedComponent :type "PrimitiveComponent Object Reference") (OtherActor :type "Actor Object Reference") (OtherComp :type "PrimitiveComponent Object Reference") (OtherBodyIndex :type Integer) (bFromSweep :type Boolean) (SweepResult :type "HitResult Structure (by ref)")))

(event `StartFire`
  (set `self.bIsBurning` true)
  (`ActorComponent.Activate` (`self.NS_Fire`) false)
  (`self.SpawnNewFire`))

(event `SpawnNewFire`
  (if (< (`self.CurrentSpread`) (`self.MaxSpreadCount`)) :!label _label
    (`|SpawnActorFromClass` "BP_FIre2_C" (`KismetMathLibrary.MakeTransform` (`KismetMathLibrary.MakeVector` (+ (.x (`self.K2_GetActorLocation`)) (`KismetMathLibrary.RandomFloatInRange` (* (`self.SpreadRangeRadius`) -1.0) (`self.SpreadRangeRadius`))) (+ (.y (`self.K2_GetActorLocation`)) (`KismetMathLibrary.RandomFloatInRange` (* (`self.SpreadRangeRadius`) -1.0) (`self.SpreadRangeRadius`))) (.z (`self.K2_GetActorLocation`))) (.rotation (`self.GetTransform`)) (.scale (`self.GetTransform`))) "Undefined" "MultiplyWithRoot" null null)
    (set `self.CurrentSpread` (+ (`self.CurrentSpread`) 1))
    (goto _label)))

(fn `UserConstructionScript`
  (`parent.UserConstructionScript`))