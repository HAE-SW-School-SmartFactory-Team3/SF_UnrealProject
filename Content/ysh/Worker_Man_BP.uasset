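; AI worker character for a fire scenario that wanders idly, flees when told to run, and dies from fire contact.
; BeginPlay adds the main UI, starts a random-point wander loop and a repeating timer that drains HP while touching fire.
; moveRun speeds it up and repeatedly paths toward nearby ActorReference targets, switching to unvisited ones when pathing fails.
; Walking, fire, escape and death states are pushed to Worker_Man_Anim_BP.
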(event `self.ReceiveBeginPlay`
  (`KismetSystemLibrary.K2_SetTimerDelegate` (delegate `CustomEvent`) 0.1 true)
  (bind _returnvalue (`|CreateWidget` "/Game/ysh/Main_UI_BP.Main_UI_BP_C"))
  (`UserWidget.AddToViewport` _returnvalue 0)
  (`self.moveIdle`))

(event `CustomEvent`
  (`KismetSystemLibrary.PrintString` (`KismetStringLibrary.Conv_IntToString` (`self.collidedFireCount`)))
  (if (<= (`self.HP`) 0)
    (bind _asworker_man_anim_bp (cast `/Game/yjs/BluePrint/Worker_Man/Worker_Man_Anim_BP` (`SkeletalMeshComponent.GetAnimInstance` (`self.Mesh`))))
    (set `/Game/yjs/BluePrint/Worker_Man/Worker_Man_Anim_BP.isDead` true _asworker_man_anim_bp)
    (`KismetSystemLibrary.Delay` 2.0)
    (`self.K2_DestroyActor` self)
    (elif (> (`self.collidedFireCount`) 0)
      (set `self.HP` (- (`self.HP`) 10)))))

(event `self.ReceiveHit`
  (params (MyComp :type "PrimitiveComponent Object Reference") (Other :type "Actor Object Reference") (OtherComp :type "PrimitiveComponent Object Reference") (bSelfMoved :type Boolean) (HitLocation :type "Vector Structure") (HitNormal :type "Vector Structure") (NormalImpulse :type "Vector Structure") (Hit :type "HitResult Structure (by ref)"))
  (cast `/Game/ysh/Vefects/Free_Fire/Shared/Particles/BP_FIre2` Other
    (:`then`
      (set `self.collidedFireCount` 1))
    (:`CastFailed`
      (set `self.collidedFireCount` 0))))

(event `moveIdle`
  (bind _asworker_man_anim_bp (cast `/Game/yjs/BluePrint/Worker_Man/Worker_Man_Anim_BP` (`SkeletalMeshComponent.GetAnimInstance` (`self.Mesh`))))
  (if (not (and (not (`/Game/yjs/BluePrint/Worker_Man/Worker_Man_Anim_BP.isEscape` _asworker_man_anim_bp)) (`self.FireOn`))) :!label _label
    (bind _asworker_man_anim_bp_2 (cast `/Game/yjs/BluePrint/Worker_Man/Worker_Man_Anim_BP` (`SkeletalMeshComponent.GetAnimInstance` (`self.Mesh`))))
    (set `/Game/yjs/BluePrint/Worker_Man/Worker_Man_Anim_BP.isWalking` true _asworker_man_anim_bp_2)
    (`|AIMoveTo` self (`NavigationSystemV1.K2_GetRandomReachablePointInRadius` (`self.K2_GetActorLocation`) 400.0 null null) null
      (:`OnSuccess`
        _)
      (:`OnFail`
        _))
    (bind _asworker_man_anim_bp_3 (cast `/Game/yjs/BluePrint/Worker_Man/Worker_Man_Anim_BP` (`SkeletalMeshComponent.GetAnimInstance` (`self.Mesh`))))
    (set `/Game/yjs/BluePrint/Worker_Man/Worker_Man_Anim_BP.isWalking` false _asworker_man_anim_bp_3)
    (`KismetSystemLibrary.Delay` 2.0)
    (if (not (`self.FireOn`))
      (goto _label))))

(event `moveRun`
  (bind _returnvalue (`KismetMathLibrary.Vector_DistanceSquared` (`CharacterMovementComponent.GetLastUpdateLocation` (`self.CharacterMovement`)) (`self.K2_GetActorLocation`)))
  (bind _asworker_man_anim_bp (cast `/Game/yjs/BluePrint/Worker_Man/Worker_Man_Anim_BP` (`SkeletalMeshComponent.GetAnimInstance` (`self.Mesh`))))
  (set `/Game/yjs/BluePrint/Worker_Man/Worker_Man_Anim_BP.isEscape` false _asworker_man_anim_bp)
  (set `/Game/yjs/BluePrint/Worker_Man/Worker_Man_Anim_BP.isFireOn` true _asworker_man_anim_bp)
  (set `CharacterMovementComponent.MaxWalkSpeed` 400.0 (`self.CharacterMovement`))
  (set `self.MinValue` 1000000000000000.0)
  (set `self.TargetIndex` 0)
  (for (_array_element _array_index) (`self.ActorReference`)
    (bind _returnvalue_2 (`KismetMathLibrary.Vector_DistanceSquared` (`CharacterMovementComponent.GetLastUpdateLocation` (`self.CharacterMovement`)) (`self.K2_GetActorLocation` _array_element)))
    (if (> (`self.MinValue`) _returnvalue_2)
      (set `self.TargetIndex` _array_index)
      (set `self.MinValue` _returnvalue_2)
      (`KismetArrayLibrary.Array_Set` (`self.Referenced`) (`self.TargetIndex`) true)
      (bind _returnvalue_3 (`AIController.MoveToLocation` (`AIBlueprintHelperLibrary.GetAIController` self) (`self.K2_GetActorLocation` (`|GetArrayItem` (`self.ActorReference`) (`self.TargetIndex`))) 500.0 false true false true null false :!label _label_2))
      (switch `EPathFollowingRequestResult` _returnvalue_3
        (:`Failed`
          (set `self.MinIndex` 0)
          (set `self.MinValue` 1000000000000000.0)
          (for (_ _array_index_2) (`self.ActorReference`)
            (if (`|GetArrayItem` (`self.Referenced`) _array_index_2)
              _
              (elif (> (`self.MinValue`) _returnvalue)
                (set `self.MinIndex` _array_index_2)
                (set `self.MinValue` _returnvalue)
                (`KismetArrayLibrary.Array_Set` (`self.Referenced`) _array_index_2 true))))
          (set `self.TargetIndex` (`self.MinIndex`))
          (`KismetSystemLibrary.Delay` 0.2)
          (goto _label_2))
        (:`AlreadyAtGoal`
          (bind _asworker_man_anim_bp_2 (cast `/Game/yjs/BluePrint/Worker_Man/Worker_Man_Anim_BP` (`SkeletalMeshComponent.GetAnimInstance` (`self.Mesh`))))
          (set `/Game/yjs/BluePrint/Worker_Man/Worker_Man_Anim_BP.isEscape` true _asworker_man_anim_bp_2)
          (set `/Game/yjs/BluePrint/Worker_Man/Worker_Man_Anim_BP.isWalking` false _asworker_man_anim_bp_2))
        (:`RequestSuccessful`
          (`KismetSystemLibrary.Delay` 0.2)
          (goto _label_2))))))

(fn `UserConstructionScript`)